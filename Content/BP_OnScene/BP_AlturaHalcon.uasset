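; Trigger volume, likely an altitude zone, that launches a hawk (BP_Halcon) attack on the player pigeon (CH_Paloma).
; On overlap, a gated DoOnce spawns the hawk high above the player and arms the attack after a random delay.
; Tick then either dives it to just beside the player or, if the hawk's NewVar0 flag is set, moves it toward its Cube.
; The spawn gate resets when an armed hawk becomes invalid.
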(event OnComponentBeginOverlap(Box)
  (params (OverlappedComponent :type Primitive%20Component%20Object%20Reference) (OtherActor :type Actor%20Object%20Reference) (OtherComp :type Primitive%20Component%20Object%20Reference) (OtherBodyIndex :type Integer) (bFromSweep :type Boolean) (SweepResult :type Hit%20Result%20Structure%20%28by%20ref%29))
  (Utilities|Casting|CastToCH_Paloma OtherActor)
  (bind _output_get (Variables|Default|SetYiempoHalcon (Math|Random|RandomInteger 8)))
  (Development|PrintString (Utilities|String|ToString(Integer) _output_get))
  (Utilities|FlowControl|DoOnce false
    (:Completed
      (bind _returnvalue (Game|SpawnActorfromClass "/Game/BP_OnScene/BP_Halcon.BP_Halcon_C" (Math|Transform|MakeTransform (+ (Transformation|GetWorldLocation (Variables|/Script/Engine.Character|GetCapsuleComponent (Variables|Default|GetRefPaloma))) "0, 0,4000.000000") "0, 0, 0" "1,1,1") "Undefined" 0 0))
      (Variables|Default|SetRefHalcon2 _returnvalue)
      (Development|PrintString "Halcon")
      (Utilities|FlowControl|Delay (Math|Conversions|ToFloat(Integer) (Variables|Default|GetYiempoHalcon)))
      (Variables|Default|SetAtaque true))))

(event EventBeginPlay
  (bind _asch_paloma (Utilities|Casting|CastToCH_Paloma (Game|GetPlayerCharacter 0)))
  (Variables|Default|SetRefPaloma _asch_paloma))

(event EventTick
  (params (DeltaSeconds :type Float%20%28single-precision%29))
  (bind _refpaloma (Variables|Default|GetRefPaloma))
  (bind _capsulecomponent (Variables|/Script/Engine.Character|GetCapsuleComponent _refpaloma))
  (bind _returnvalue (Transformation|GetWorldLocation _capsulecomponent))
  (if (Variables|Default|GetAtaque)
    (Utilities|IsValid (Variables|Default|GetRefHalcon2)
      (:Is%20Valid
        (if (Variables|/Game/BP_OnScene/BP_Halcon.BP_Halcon_C|GetNewVar_0 (Variables|Default|GetRefHalcon2))
          (Utilities|FlowControl|Delay 0.25)
          (Utilities|FlowControl|DoOnce false
            (:Completed
              (Utilities|IsValid (Variables|Default|GetRefHalcon2)
                (:Is%20Valid
                  (Components|MoveComponentTo (Variables|/Script/Engine.Actor|GetRootComponent (Variables|Default|GetRefHalcon2)) (Transformation|GetWorldLocation (Variables|/Game/BP_OnScene/BP_Halcon.BP_Halcon_C|GetCube (Variables|Default|GetRefHalcon2))) "0, 0, 0" false false 1.0 false)))))
          (else
            (Components|MoveComponentTo (Variables|/Script/Engine.Actor|GetRootComponent (Variables|Default|GetRefHalcon2)) (+ _returnvalue "50.000000,0.000000,-30.000000") (Transformation|GetWorldRotation (Variables|/Game/BluePrints/Paloma/CH_Paloma.CH_Paloma_C|GetArrow1 (Variables|Default|GetRefPaloma))) false false 0.3 false)
            (Variables|Default|SetAtaque false))))
      (:Is%20Not%20Valid
        (Utilities|FlowControl|DoOnce false) ; enters at Reset
      ))))

(fn ConstructionScript)