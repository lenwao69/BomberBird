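; BP_Halcon is a hawk encounter that puts the player's pigeon (CH_Paloma) through an escape-or-die moment.
; The camera sphere blends to BP_CameraMuerte and once runs a randomly picked, near-identical macro, reading the warning widget's Muerte flag after 1.5s.
; Escape awards points and opens a Tick gate that restores the view and destroys the hawk; death triggers game over.
; The death sphere plays attack sounds and starts per-tick camera movement.
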(event OnComponentBeginOverlap(EsferaMuerte)
  (params (OverlappedComponent :type Primitive%20Component%20Object%20Reference) (OtherActor :type Actor%20Object%20Reference) (OtherComp :type Primitive%20Component%20Object%20Reference) (OtherBodyIndex :type Integer) (bFromSweep :type Boolean) (SweepResult :type Hit%20Result%20Structure%20%28by%20ref%29))
  (bind _ref_pc_paloma (Variables|Default|GetRef_PC_Paloma))
  (bind _volumensonidos (Variables|/Game/BluePrints/Paloma/PC_Paloma.PC_Paloma_C|GetVolumenSonidos _ref_pc_paloma))
  (Utilities|Casting|CastToCH_Paloma OtherActor)
  (Audio|PlaySound2D "/Game/Sonido/WesternSound.WesternSound" _volumensonidos 1.0 0.0 0 0)
  (Utilities|FlowControl|Delay 0.2)
  (Audio|PlaySound2D "/Game/Sonido/AttackHawk.AttackHawk" _volumensonidos 1.0 0.0 0 0)
  (Variables|Default|SetNewVar_0 true))

(event OnComponentBeginOverlap(EsferaCamaraMuerte)
  (params (OverlappedComponent :type Primitive%20Component%20Object%20Reference) (OtherActor :type Actor%20Object%20Reference) (OtherComp :type Primitive%20Component%20Object%20Reference) (OtherBodyIndex :type Integer) (bFromSweep :type Boolean) (SweepResult :type Hit%20Result%20Structure%20%28by%20ref%29))
  (bind _ref_pc_paloma (Variables|Default|GetRef_PC_Paloma))
  (bind _ref_ch_paloma (Variables|Default|GetRef_Ch_paloma))
  (bind _ref_pc_paloma_2 (Variables|Default|GetRef_PC_Paloma))
  (bind _ref_pc_paloma_3 (Variables|Default|GetRef_PC_Paloma))
  (Utilities|Casting|CastToCH_Paloma OtherActor)
  (Game|Player|SetViewTargetwithBlend (Game|GetPlayerController 0) (Variables|Default|GetRefCAmaraMuerte) 0.6 "VTBlend_Linear" 0.0 false)
  (Utilities|FlowControl|DoOnce false
    (:Completed
      (bind _output_get (Variables|Default|SetNumeroAzar (Math|Random|RandomInteger 4)))
      (switch int _output_get
        (:0
          (Utilities|AbrirWidget1
            (:then
              (Default|SumarPuntos _ref_pc_paloma 0.0 (Variables|/Game/BluePrints/Paloma/PC_Paloma.PC_Paloma_C|GetPuntosHuida _ref_pc_paloma) 0.0 :!label _label)
              (Audio|PlaySound2D "/Game/Sonido/Escapar.Escapar" (Variables|/Game/BluePrints/Paloma/PC_Paloma.PC_Paloma_C|GetVolumenSonidos _ref_pc_paloma) 1.0 0.0 0 0)
              (Utilities|FlowControl|Gate true) ; enters at Open
            )
            (:then2
              (Audio|PlaySound2D "/Game/Sonido/MuertePaloma.MuertePaloma" (Variables|/Game/BluePrints/Paloma/PC_Paloma.PC_Paloma_C|GetVolumenSonidos _ref_pc_paloma) 1.0 0.0 0 0 :!label _label_2)
              (Variables|Default|SetNewVar_0 true)
              (Rendering|SetVisibility (Variables|/Script/Engine.Character|GetMesh _ref_ch_paloma) false false)
              (Rendering|SetVisibility (Variables|/Game/BluePrints/Paloma/CH_Paloma.CH_Paloma_C|GetGorro _ref_ch_paloma) false false)
              (Default|GuardarDatos _ref_pc_paloma_3)
              (Components|Activation|Deactivate (Variables|/Script/Engine.Character|GetCharacterMovement _ref_ch_paloma))
              (Default|GameOver _ref_pc_paloma_3)
              (Utilities|FlowControl|Delay 5.0)
              (Variables|Default|SetNewVar_0 false)
              (UserInterface|Viewport|AddtoViewport (Variables|Default|GetRefMenuMuerte) 0))))
        (:1
          (Utilities|AbrirWidget2
            (:then
              (goto _label))
            (:then2
              (goto _label_2))))
        (:2
          (Utilities|AbrirWidget3
            (:then
              (goto _label))
            (:then2
              (goto _label_2))))
        (:3
          (Utilities|AbrirWidget4
            (:then
              (goto _label))
            (:then2
              (goto _label_2))))
        (:4
          (Utilities|AbrirWidget5
            (:then
              (goto _label))
            (:then2
              (goto _label_2))))))))

(event Custom|Close
  (bind _ref_pc_paloma (Variables|Default|GetRef_PC_Paloma))
  (Utilities|FlowControl|Gate true) ; enters at Close
)

(event EventBeginPlay
  (bind _asch_paloma (Utilities|Casting|CastToCH_Paloma (Game|GetPlayerCharacter 0)))
  (Variables|Default|SetRef_Ch_paloma _asch_paloma)
  (bind _outactors (Actor|GetAllActorsOfClass "/Game/BluePrints/Paloma/BP_CameraMuerte.BP_CameraMuerte_C"))
  (Variables|Default|SetRefCamaraMuerte (Utilities|Array|Get(acopy) _outactors))
  (bind _returnvalue (UserInterface|CreateWidget "/Game/Widgets/HUD/Widg_Aviso.Widg_Aviso_C"))
  (Variables|Default|SetWidgetAviso1 _returnvalue)
  (bind _outactors_2 (Actor|GetAllActorsOfClass "/Game/BluePrints/Paloma/PC_Paloma.PC_Paloma_C"))
  (Variables|Default|SetRef_PC_Paloma (Utilities|Array|Get(acopy) _outactors_2))
  (bind _returnvalue_2 (UserInterface|CreateWidget "/Game/Widgets/HUD/Widg_FinPartida.Widg_FinPartida_C"))
  (Variables|Default|SetRefMenuMuerte _returnvalue_2)
  (bind _returnvalue_3 (UserInterface|CreateWidget "/Game/Widgets/Publicidad.Publicidad_C"))
  (Variables|Default|SetRef_publicidad _returnvalue_3))

(event EventTick
  (params (DeltaSeconds :type Float%20%28single-precision%29))
  (bind _ref_pc_paloma (Variables|Default|GetRef_PC_Paloma))
  (Utilities|FlowControl|Sequence
    (:then_0
      (Utilities|FlowControl|Gate true
        (:Exit
          (Utilities|FlowControl|Sequence
            (:then_0
              (Game|Player|SetViewTargetwithBlend (Game|GetPlayerController 0) (Variables|Default|GetRef_Ch_paloma) 0.6 "VTBlend_Linear" 0.0 false)
              (Actor|DestroyActor)
              (Default|Huir (Variables|Default|GetRef_Ch_paloma))
              (Utilities|IsValid _ref_pc_paloma
                (:Is%20Valid
                  (Variables|/Game/BluePrints/Paloma/PC_Paloma.PC_Paloma_C|SetMoverAlante _ref_pc_paloma true))))
            (:then_1
              (Utilities|FlowControl|Delay 2.0)
              (CallFunction|Close))))))
    (:then_1
      (if (Variables|Default|GetNewVar_0)
        (Default|Moverse (Variables|Default|GetRefCamaraMuerte))))))

(fn ConstructionScript)