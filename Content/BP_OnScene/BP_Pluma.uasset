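; BP_Pluma is a feather pickup that grants turbo to the pigeon player.
; The first CH_Paloma overlap with its box calls TurboGetPluma on the PC_Paloma controller, then destroys the feather after a short delay.
; It then tells the first BP_SpawnPluma found at BeginPlay to respawn.
; A vertical mesh timeline is unwired, and the Widg_Vida widget created at BeginPlay is only stored.
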(event OnComponentBeginOverlap(Box)
  (params (OverlappedComponent :type Primitive%20Component%20Object%20Reference) (OtherActor :type Actor%20Object%20Reference) (OtherComp :type Primitive%20Component%20Object%20Reference) (OtherBodyIndex :type Integer) (bFromSweep :type Boolean) (SweepResult :type Hit%20Result%20Structure%20%28by%20ref%29))
  (bind _refspawnpluma2 (Variables|Default|GetRefSpawnpluma2))
  (Utilities|Casting|CastToCH_Paloma OtherActor)
  (Utilities|FlowControl|DoOnce false
    (:Completed
      (Default|TurboGetPluma (Variables|Default|GetRefPaloma))
      (Utilities|FlowControl|Delay 0.2)
      (Actor|DestroyActor)
      (Utilities|IsValid _refspawnpluma2
        (:Is%20Valid
          (Default|VolverARespawnear _refspawnpluma2))))))

(event EventBeginPlay
  (bind _aspc_paloma (Utilities|Casting|CastToPC_Paloma (Game|GetPlayerController 0)))
  (Variables|Default|SetRefPaloma _aspc_paloma)
  (bind _returnvalue (UserInterface|CreateWidget "/Game/Widgets/HUD/Widg_Vida.Widg_Vida_C"))
  (Variables|Default|SetNewVar_1 _returnvalue)
  (bind _outactors (Actor|GetAllActorsOfClass "/Game/BP_OnScene/BP_SpawnPluma.BP_SpawnPluma_C"))
  (Variables|Default|SetRefSpawnpluma2 (Utilities|Array|Get(acopy) _outactors)))

(fn ConstructionScript)