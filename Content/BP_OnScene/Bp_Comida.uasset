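; Food spot where the player pigeon (CH_Paloma) perches to refill its ammo.
; Sphere overlap toggles the perched flag here and on PC_Paloma, and turns off the pigeon's controller-yaw rotation while perched.
; Entering starts a looping timer that, while perched, adds ammo to the controller until it reaches the cap and updates the Widg_Vida ammo bar.
; The timer is never cleared on exit, only gated by the flag.
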(event OnComponentBeginOverlap(Sphere)
  (params (OverlappedComponent :type Primitive%20Component%20Object%20Reference) (OtherActor :type Actor%20Object%20Reference) (OtherComp :type Primitive%20Component%20Object%20Reference) (OtherBodyIndex :type Integer) (bFromSweep :type Boolean) (SweepResult :type Hit%20Result%20Structure%20%28by%20ref%29))
  (Utilities|Casting|CastToCH_Paloma OtherActor)
  (Variables|Default|SetB_Paloma_Posada true)
  (bind _aspc_paloma (Utilities|Casting|CastToPC_Paloma (Game|GetPlayerController 0)))
  (Variables|/Game/BluePrints/Paloma/PC_Paloma.PC_Paloma_C|SetPalomaPosada _aspc_paloma true)
  (Variables|/Script/Engine.Pawn|SetbUseControllerRotationYaw (Variables|Default|GetRefPaloma) false)
  (CallFunction|CustomEvent0))

(event OnComponentEndOverlap(Sphere)
  (params (OverlappedComponent :type Primitive%20Component%20Object%20Reference) (OtherActor :type Actor%20Object%20Reference) (OtherComp :type Primitive%20Component%20Object%20Reference) (OtherBodyIndex :type Integer))
  (Utilities|Casting|CastToCH_Paloma OtherActor)
  (Variables|Default|SetB_Paloma_Posada false)
  (bind _aspc_paloma (Utilities|Casting|CastToPC_Paloma (Game|GetPlayerController 0)))
  (Variables|/Game/BluePrints/Paloma/PC_Paloma.PC_Paloma_C|SetPalomaPosada _aspc_paloma false)
  (Variables|/Script/Engine.Pawn|SetbUseControllerRotationYaw (Variables|Default|GetRefPaloma) true))

(event Custom|CustomEvent_0
  (Utilities|Time|SetTimerbyEvent (delegate Custom|CustomEvent_1) 1.3 true))

(event Custom|CustomEvent_1
  (bind _refmunicionpaloma (Variables|Default|GetREfMunicionpaloma))
  (bind _progress_cacas (Variables|/Game/Widgets/HUD/Widg_Vida.Widg_Vida_C|GetProgress_Cacas _refmunicionpaloma))
  (if (Variables|Default|GetB_Paloma_Posada)
    (bind _aspc_paloma (Utilities|Casting|CastToPC_Paloma (Game|GetPlayerController 0)))
    (if (not (>= (Variables|/Game/BluePrints/Paloma/PC_Paloma.PC_Paloma_C|GetFl_Municion _aspc_paloma) 1e+02))
      (Variables|/Game/BluePrints/Paloma/PC_Paloma.PC_Paloma_C|SetFl_Municion _aspc_paloma (+ (Variables|/Game/BluePrints/Paloma/PC_Paloma.PC_Paloma_C|GetFl_Municion _aspc_paloma) (Variables|Default|GetFl_Suma_Municion)))
      (Utilities|IsValid _progress_cacas
        (:Is%20Valid
          (Progress|SetPercent _progress_cacas (/ (Variables|/Game/BluePrints/Paloma/PC_Paloma.PC_Paloma_C|GetFl_Municion _aspc_paloma) 1e+02)))))))

(event EventBeginPlay
  (bind _outactors (Actor|GetAllActorsOfClass "/Game/BluePrints/Paloma/CH_Paloma.CH_Paloma_C"))
  (Variables|Default|SetRefPaloma (Utilities|Array|Get(acopy) _outactors))
  (bind _foundwidgets (Widget|GetAllWidgetsOfClass "/Game/Widgets/HUD/Widg_Vida.Widg_Vida_C" false))
  (Variables|Default|SetREfMunicionpaloma (Utilities|Array|Get(acopy) _foundwidgets)))

(fn ConstructionScript)