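; TareaCamino2 is a Behavior Tree task that walks an AI along a spline path.
; On execute it gets the BP_Spline2 spline from the Camino2 blackboard key and resets the travelled distance.
; Each tick it advances the distance by a fixed step, independent of delta time, and calls SimpleMoveToLocation to that spline point.
; It finishes successfully when the distance nears the spline's length.
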(event EventReceiveExecuteAI
  (params (OwnerController :type AI%20Controller%20Object%20Reference) (ControlledPawn :type Pawn%20Object%20Reference))
  (Variables|Default|SetrefSpline2a (Variables|/Game/BluePrints/Cato2/BP_Spline2.BP_Spline2_C|GetSpline (.AsBP%20Spline%202 (Utilities|Casting|CastToBP_Spline2 (Class|BTFunctionLibrary|GetBlackboardValueasObject (Variables|Default|GetCamino2))))))
  (Variables|Default|Setdistancia 0.0))

(event EventReceiveTickAI
  (params (OwnerController :type AI%20Controller%20Object%20Reference) (ControlledPawn :type Pawn%20Object%20Reference) (DeltaSeconds :type Float%20%28single-precision%29))
  (bind _output_get (Variables|Default|Setdistancia (+ (Variables|Default|Getdistancia) 8.0)))
  (AI|Navigation|SimpleMovetoLocation OwnerController (Spline|GetLocationatDistanceAlongSpline (Variables|Default|GetrefSpline2a) _output_get "World"))
  (if (Math|Float|NearlyEqual(Float) (Spline|GetSplineLength (Variables|Default|GetrefSpline2a)) _output_get 15.0)
    (AI|BehaviorTree|FinishExecute true)))