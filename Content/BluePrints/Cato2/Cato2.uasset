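; Cato2 is a cat enemy whose trigger volumes threaten the player pigeon (CH_Paloma).
; SaltoAtaque overlap screams and pulses an attack flag; CajaCamaraMuerte overlap blends to BP_CameraMuerte and randomly picks among near-identical AbrirWidget macros showing a warning widget.
; After two seconds, its Muerte flag selects death (effects, save, game over, paused end menu) or escape (points, camera return, gated upward push).
; Tick drives that push and the moving death camera.
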(event OnComponentEndOverlap(SaltoAtaque)
  (params (OverlappedComponent :type Primitive%20Component%20Object%20Reference) (OtherActor :type Actor%20Object%20Reference) (OtherComp :type Primitive%20Component%20Object%20Reference) (OtherBodyIndex :type Integer))
  (Utilities|Casting|CastToCH_Paloma OtherActor)
  (Variables|Default|SetAtaque_0 false))

(event OnComponentBeginOverlap(CajaCamaraMuerte)
  (params (OverlappedComponent :type Primitive%20Component%20Object%20Reference) (OtherActor :type Actor%20Object%20Reference) (OtherComp :type Primitive%20Component%20Object%20Reference) (OtherBodyIndex :type Integer) (bFromSweep :type Boolean) (SweepResult :type Hit%20Result%20Structure%20%28by%20ref%29))
  (bind _refchpaloma (Variables|Default|GetRefCHpaloma))
  (bind _refchpaloma_2 (Variables|Default|GetRefCHpaloma))
  (bind _refchpaloma_3 (Variables|Default|GetRefCHpaloma))
  (bind _pcpalomaref (Variables|Default|GetPCPALOMAREF))
  (bind _pcpalomaref_2 (Variables|Default|GetPCPALOMAREF))
  (bind _charactermovement (Variables|/Script/Engine.Character|GetCharacterMovement _refchpaloma_2))
  (Utilities|Casting|CastToCH_Paloma OtherActor)
  (Utilities|FlowControl|DoOnce false
    (:Completed
      (Game|Player|SetViewTargetwithBlend (Game|GetPlayerController 0) (Variables|Default|GetRefCameraMuerte) 0.6 "VTBlend_Linear" 0.0 false)
      (Utilities|FlowControl|Sequence
        (:then_0
          (bind _output_get (Variables|Default|SetNuevoNum (Math|Random|RandomInteger 4)))
          (Utilities|FlowControl|Delay 0.2)
          (switch int _output_get
            (:0
              (Utilities|AbrirWidget1
                (:then
                  (Variables|/Game/BluePrints/Paloma/PC_Paloma.PC_Paloma_C|SetMoverAlante _pcpalomaref true :!label _label)
                  (Variables|/Script/Engine.CharacterMovementComponent|SetMaxFlySpeed _charactermovement 4e+02)
                  (Components|Activation|Activate _charactermovement false)
                  (Default|SumarPuntos _pcpalomaref 0.0 (Variables|/Game/BluePrints/Paloma/PC_Paloma.PC_Paloma_C|GetPuntosHuida _pcpalomaref) 0.0)
                  (Audio|PlaySound2D "/Game/Sonido/Escapar.Escapar" (Variables|/Game/BluePrints/Paloma/PC_Paloma.PC_Paloma_C|GetVolumenSonidos _pcpalomaref) 1.0 0.0 0 0)
                  (Utilities|FlowControl|Gate true) ; enters at Open
                )
                (:then2
                  (Audio|PlaySound2D "/Game/Sonido/MuertePaloma.MuertePaloma" (Variables|/Game/BluePrints/Paloma/PC_Paloma.PC_Paloma_C|GetVolumenSonidos _pcpalomaref_2) 1.0 0.0 0 0 :!label _label_2)
                  (Variables|Default|SetNewVar_1 true)
                  (Variables|/Game/BluePrints/Paloma/PC_Paloma.PC_Paloma_C|SetMoverAlante _pcpalomaref_2 false)
                  (Rendering|SetVisibility (Variables|/Script/Engine.Character|GetMesh _refchpaloma) false false)
                  (Rendering|SetVisibility (Variables|/Game/BluePrints/Paloma/CH_Paloma.CH_Paloma_C|GetGorro _refchpaloma) false false)
                  (Default|GuardarDatos (Variables|Default|GetPCPALOMAREF))
                  (Default|GameOver (Variables|Default|GetPCPALOMAREF))
                  (Utilities|FlowControl|Delay 5.0)
                  (Variables|Default|SetNewVar_1 false)
                  (UserInterface|Viewport|AddtoViewport (Variables|Default|GetRefMEnuMuertee) 0)
                  (Game|SetGamePaused true))))
            (:1
              (Utilities|AbrirWidget2
                (:then
                  (goto _label))
                (:then2
                  (goto _label_2))))
            (:2
              (Utilities|AbrirWidget3
                (:then
                  (goto _label))
                (:then2
                  (goto _label_2))))
            (:3
              (Utilities|AbrirWidget4
                (:then
                  (goto _label))
                (:then2
                  (goto _label_2))))
            (:4
              (Utilities|AbrirWidget5
                (:then
                  (goto _label))
                (:then2
                  (goto _label_2))))))))))

(event OnComponentBeginOverlap(EsferaCamaraMuerte)
  (params (OverlappedComponent :type Primitive%20Component%20Object%20Reference) (OtherActor :type Actor%20Object%20Reference) (OtherComp :type Primitive%20Component%20Object%20Reference) (OtherBodyIndex :type Integer) (bFromSweep :type Boolean) (SweepResult :type Hit%20Result%20Structure%20%28by%20ref%29)))

(event OnComponentBeginOverlap(SaltoAtaque)
  (params (OverlappedComponent :type Primitive%20Component%20Object%20Reference) (OtherActor :type Actor%20Object%20Reference) (OtherComp :type Primitive%20Component%20Object%20Reference) (OtherBodyIndex :type Integer) (bFromSweep :type Boolean) (SweepResult :type Hit%20Result%20Structure%20%28by%20ref%29))
  (Utilities|Casting|CastToCH_Paloma OtherActor)
  (Utilities|FlowControl|DoOnce false :!label _label
    (:Completed
      (Variables|Default|SetAtaque_0 true)
      (Audio|PlaySound2D "/Game/Sonido/Gritocato.Gritocato" 1.0 1.0 0.0 0 0)
      (Utilities|FlowControl|Delay 1.0)
      (Variables|Default|SetAtaque_0 false)
      (goto _label Reset))))

(event EventBeginPlay
  (bind _outactors (Actor|GetAllActorsOfClass "/Game/BluePrints/Paloma/BP_CameraMuerte.BP_CameraMuerte_C"))
  (Variables|Default|SetRefCameraMuerte (Utilities|Array|Get(acopy) _outactors))
  (bind _returnvalue (UserInterface|CreateWidget "/Game/Widgets/HUD/Widg_Aviso.Widg_Aviso_C"))
  (Variables|Default|SetAvisoWidget _returnvalue)
  (bind _outactors_2 (Actor|GetAllActorsOfClass "/Game/BluePrints/Paloma/CH_Paloma.CH_Paloma_C"))
  (Variables|Default|SetRefCHpaloma (Utilities|Array|Get(acopy) _outactors_2))
  (bind _aspc_paloma (Utilities|Casting|CastToPC_Paloma (Game|GetPlayerController 0)))
  (Variables|Default|SetPCPALOMAREF _aspc_paloma)
  (bind _returnvalue_2 (UserInterface|CreateWidget "/Game/Widgets/HUD/Widg_FinPartida.Widg_FinPartida_C"))
  (Variables|Default|SetRefMEnuMuertee _returnvalue_2)
  (bind _returnvalue_3 (UserInterface|CreateWidget "/Game/Widgets/Publicidad.Publicidad_C"))
  (Variables|Default|Setpublicidad _returnvalue_3))

(event EventTick
  (params (DeltaSeconds :type Float%20%28single-precision%29))
  (bind _refchpaloma (Variables|Default|GetRefCHpaloma))
  (bind _refchpaloma_2 (Variables|Default|GetRefCHpaloma))
  (bind _refchpaloma_3 (Variables|Default|GetRefCHpaloma))
  (bind _pcpalomaref (Variables|Default|GetPCPALOMAREF))
  (bind _pcpalomaref_2 (Variables|Default|GetPCPALOMAREF))
  (bind _charactermovement (Variables|/Script/Engine.Character|GetCharacterMovement _refchpaloma_2))
  (Utilities|FlowControl|Sequence
    (:then_0
      (if (Variables|Default|GetNewVar_1)
        (Default|Moverse (Variables|Default|GetRefCameraMuerte))))
    (:then_1
      (Utilities|FlowControl|Gate true :!label _label
        (:Exit
          (Variables|/Game/BluePrints/Paloma/PC_Paloma.PC_Paloma_C|SetMoverAlante (Variables|Default|GetPCPALOMAREF) true)
          (Pawn|Input|AddMovementInput _refchpaloma_3 (Math|Vector|GetUpVector (Math|Rotator|MakeRotator 0.0 0.0 (.yaw (Pawn|GetControlRotation _refchpaloma_3 :!class /Script/Engine.Pawn)))) 1.0 false)
          (Utilities|FlowControl|Sequence
            (:then_0
              (Game|Player|SetViewTargetwithBlend (Game|GetPlayerController 0) (Variables|Default|GetRefCHpaloma) 0.6 "VTBlend_Linear" 0.0 false)
              (Utilities|FlowControl|DoOnce false) ; enters at Reset
            )
            (:then_1
              (Utilities|FlowControl|Delay 2.0)
              (goto _label Close))))))))

(fn ConstructionScript)