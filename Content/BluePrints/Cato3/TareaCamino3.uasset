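; Behavior tree task that walks an AI-controlled pawn along a BP_Spline3 path.
; On execute it reads the spline actor from the Camino2 blackboard key and resets the travelled distance.
; Each tick it advances the distance by a fixed, frame-rate-dependent step and calls SimpleMoveToLocation on that spline point.
; It finishes successfully when the distance nears the spline's length; a debug point draw is left unconnected.
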(event EventReceiveExecuteAI
  (params (OwnerController :type AI%20Controller%20Object%20Reference) (ControlledPawn :type Pawn%20Object%20Reference))
  (Variables|Default|SetRefSpline3 (Variables|/Game/BluePrints/Cato3/BP_Spline3.BP_Spline3_C|GetSpline (.AsBP%20Spline%203 (Utilities|Casting|CastToBP_Spline3 (Class|BTFunctionLibrary|GetBlackboardValueasObject (Variables|Default|GetCamino2))))))
  (Variables|Default|Setdistancia 0.0))

(event EventReceiveTickAI
  (params (OwnerController :type AI%20Controller%20Object%20Reference) (ControlledPawn :type Pawn%20Object%20Reference) (DeltaSeconds :type Float%20%28single-precision%29))
  (bind _output_get (Variables|Default|Setdistancia (+ (Variables|Default|Getdistancia) 8.0)))
  (AI|Navigation|SimpleMovetoLocation OwnerController (Spline|GetLocationatDistanceAlongSpline (Variables|Default|GetRefSpline3) _output_get "World"))
  (if (Math|Float|NearlyEqual(Float) (Spline|GetSplineLength (Variables|Default|GetRefSpline3)) _output_get 15.0)
    (AI|BehaviorTree|FinishExecute true)))