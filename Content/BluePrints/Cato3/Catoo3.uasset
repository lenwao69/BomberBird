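; Cat enemy that ambushes the player pigeon (CH_Paloma), with a jump-attack trigger that briefly sets Ataque and plays a scream.
; Its camera box blends to BP_CameraMuerte and randomly runs one of several near-identical macros showing a two-second warning widget.
; The widget's Muerte flag decides between escape (points, brief upward push, camera return) and death (particles, save, game over, paused menu).
; Tick drives the death camera and the gated escape push.
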(event OnComponentEndOverlap(SaltoAtaque)
  (params (OverlappedComponent :type Primitive%20Component%20Object%20Reference) (OtherActor :type Actor%20Object%20Reference) (OtherComp :type Primitive%20Component%20Object%20Reference) (OtherBodyIndex :type Integer))
  (Utilities|Casting|CastToCH_Paloma OtherActor)
  (Variables|Default|SetAtaque false))

(event OnComponentBeginOverlap(CajaCamaraMuerte)
  (params (OverlappedComponent :type Primitive%20Component%20Object%20Reference) (OtherActor :type Actor%20Object%20Reference) (OtherComp :type Primitive%20Component%20Object%20Reference) (OtherBodyIndex :type Integer) (bFromSweep :type Boolean) (SweepResult :type Hit%20Result%20Structure%20%28by%20ref%29))
  (bind _pc_paloma_ref (Variables|Default|GetPc_paloma_ref))
  (bind _refpaloma (Variables|Default|GetRefPaloma))
  (bind _pc_paloma_ref_2 (Variables|Default|GetPc_paloma_ref))
  (bind _refpaloma_2 (Variables|Default|GetRefPaloma))
  (bind _refpaloma_3 (Variables|Default|GetRefPaloma))
  (bind _charactermovement (Variables|/Script/Engine.Character|GetCharacterMovement _refpaloma_3))
  (Utilities|Casting|CastToCH_Paloma OtherActor)
  (Utilities|FlowControl|DoOnce false
    (:Completed
      (Game|Player|SetViewTargetwithBlend (Game|GetPlayerController 0) (Variables|Default|GetRefCAmaraMuerte) 0.6 "VTBlend_Linear" 0.0 false)
      (Utilities|FlowControl|Sequence
        (:then_0
          (bind _output_get (Variables|Default|SetNumeroAzar (Math|Random|RandomInteger 4)))
          (Utilities|FlowControl|Delay 0.2)
          (switch int _output_get
            (:0
              (Utilities|AbrirWidget1
                (:then
                  (Variables|/Game/BluePrints/Paloma/PC_Paloma.PC_Paloma_C|SetMoverAlante _pc_paloma_ref_2 true :!label _label)
                  (Variables|/Script/Engine.CharacterMovementComponent|SetMaxFlySpeed _charactermovement 4e+02)
                  (Components|Activation|Activate _charactermovement false)
                  (Default|SumarPuntos _pc_paloma_ref_2 0.0 (Variables|/Game/BluePrints/Paloma/PC_Paloma.PC_Paloma_C|GetPuntosHuida _pc_paloma_ref_2) 0.0)
                  (Audio|PlaySound2D "/Game/Sonido/Escapar.Escapar" (Variables|/Game/BluePrints/Paloma/PC_Paloma.PC_Paloma_C|GetVolumenSonidos _pc_paloma_ref_2) 1.0 0.0 0 0)
                  (Utilities|FlowControl|Gate true) ; enters at Open
                )
                (:then2
                  (Audio|PlaySound2D "/Game/Sonido/MuertePaloma.MuertePaloma" (Variables|/Game/BluePrints/Paloma/PC_Paloma.PC_Paloma_C|GetVolumenSonidos _pc_paloma_ref) 1.0 0.0 0 0 :!label _label_2)
                  (Variables|Default|SetNewVar_0 true)
                  (Variables|/Game/BluePrints/Paloma/PC_Paloma.PC_Paloma_C|SetMoverAlante _pc_paloma_ref false)
                  (Rendering|SetVisibility (Variables|/Script/Engine.Character|GetMesh _refpaloma_2) false false)
                  (Rendering|SetVisibility (Variables|/Game/BluePrints/Paloma/CH_Paloma.CH_Paloma_C|GetGorro _refpaloma_2) false false)
                  (Default|GuardarDatos _pc_paloma_ref)
                  (Default|GameOver (Variables|Default|GetPc_paloma_ref))
                  (Utilities|FlowControl|Delay 5.0)
                  (Variables|Default|SetNewVar_0 false)
                  (UserInterface|Viewport|AddtoViewport (Variables|Default|GetRefMenuMuerte) 0)
                  (Game|SetGamePaused true))))
            (:1
              (Utilities|AbrirWidget2
                (:then
                  (goto _label))
                (:then2
                  (goto _label_2))))
            (:2
              (Utilities|AbrirWidget3
                (:then
                  (goto _label))
                (:then2
                  (goto _label_2))))
            (:3
              (Utilities|AbrirWidget4
                (:then
                  (goto _label))
                (:then2
                  (goto _label_2))))
            (:4
              (Utilities|AbrirWidget5
                (:then
                  (goto _label))
                (:then2
                  (goto _label_2))))))))))

(event OnComponentBeginOverlap(EsferaCamaraMuerte)
  (params (OverlappedComponent :type Primitive%20Component%20Object%20Reference) (OtherActor :type Actor%20Object%20Reference) (OtherComp :type Primitive%20Component%20Object%20Reference) (OtherBodyIndex :type Integer) (bFromSweep :type Boolean) (SweepResult :type Hit%20Result%20Structure%20%28by%20ref%29)))

(event OnComponentBeginOverlap(SaltoAtaque)
  (params (OverlappedComponent :type Primitive%20Component%20Object%20Reference) (OtherActor :type Actor%20Object%20Reference) (OtherComp :type Primitive%20Component%20Object%20Reference) (OtherBodyIndex :type Integer) (bFromSweep :type Boolean) (SweepResult :type Hit%20Result%20Structure%20%28by%20ref%29))
  (Utilities|Casting|CastToCH_Paloma OtherActor)
  (Utilities|FlowControl|DoOnce false :!label _label
    (:Completed
      (Variables|Default|SetAtaque true)
      (Audio|PlaySound2D "/Game/Sonido/Gritocato.Gritocato" (Variables|/Game/BluePrints/Paloma/PC_Paloma.PC_Paloma_C|GetPuntosHuida (Variables|Default|GetPc_paloma_ref)) 1.0 0.0 0 0)
      (Utilities|FlowControl|Delay 1.0)
      (Variables|Default|SetAtaque false)
      (goto _label Reset))))

(event EventBeginPlay
  (bind _outactors (Actor|GetAllActorsOfClass "/Game/BluePrints/Paloma/BP_CameraMuerte.BP_CameraMuerte_C"))
  (Variables|Default|SetRefCAmaraMuerte (Utilities|Array|Get(acopy) _outactors))
  (bind _returnvalue (UserInterface|CreateWidget "/Game/Widgets/HUD/Widg_Aviso.Widg_Aviso_C"))
  (Variables|Default|SetWidgetaviso _returnvalue)
  (bind _outactors_2 (Actor|GetAllActorsOfClass "/Game/BluePrints/Paloma/CH_Paloma.CH_Paloma_C"))
  (Variables|Default|SetRefPaloma (Utilities|Array|Get(acopy) _outactors_2))
  (bind _aspc_paloma (Utilities|Casting|CastToPC_Paloma (Game|GetPlayerController 0)))
  (Variables|Default|SetPc_paloma_ref _aspc_paloma)
  (bind _returnvalue_2 (UserInterface|CreateWidget "/Game/Widgets/HUD/Widg_FinPartida.Widg_FinPartida_C"))
  (Variables|Default|SetRefMenuMuerte _returnvalue_2)
  (bind _returnvalue_3 (UserInterface|CreateWidget "/Game/Widgets/Publicidad.Publicidad_C"))
  (Variables|Default|SetPublicidad _returnvalue_3))

(event EventTick
  (params (DeltaSeconds :type Float%20%28single-precision%29))
  (bind _pc_paloma_ref (Variables|Default|GetPc_paloma_ref))
  (bind _refpaloma (Variables|Default|GetRefPaloma))
  (bind _pc_paloma_ref_2 (Variables|Default|GetPc_paloma_ref))
  (bind _refpaloma_2 (Variables|Default|GetRefPaloma))
  (bind _refpaloma_3 (Variables|Default|GetRefPaloma))
  (bind _charactermovement (Variables|/Script/Engine.Character|GetCharacterMovement _refpaloma_3))
  (Utilities|FlowControl|Sequence
    (:then_0
      (if (Variables|Default|GetNewVar_0)
        (Default|Moverse (Variables|Default|GetRefCAmaraMuerte))))
    (:then_1
      (Utilities|FlowControl|Gate true :!label _label
        (:Exit
          (Variables|/Game/BluePrints/Paloma/PC_Paloma.PC_Paloma_C|SetMoverAlante (Variables|Default|GetPc_paloma_ref) true)
          (Pawn|Input|AddMovementInput _refpaloma (Math|Vector|GetUpVector (Math|Rotator|MakeRotator 0.0 0.0 (.yaw (Pawn|GetControlRotation _refpaloma :!class /Script/Engine.Pawn)))) 1.0 false)
          (Utilities|FlowControl|Sequence
            (:then_0
              (Game|Player|SetViewTargetwithBlend (Game|GetPlayerController 0) (Variables|Default|GetRefPaloma) 0.6 "VTBlend_Linear" 0.0 false)
              (Utilities|FlowControl|DoOnce false) ; enters at Reset
            )
            (:then_1
              (Utilities|FlowControl|Delay 2.0)
              (goto _label Close))))))))

(fn ConstructionScript)