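; Pigeon poop projectile actor whose look follows the hat equipped on the PC_Paloma player controller, and which destroys itself a short while after spawning.
; On BeginPlay it caches that controller, then the Proyectiles macro reads the hat's DataTable_Gorros row to set the skeletal mesh, with index-based overrides for material, ball meshes or animated default.
; RotacionCamera pitches the mesh through a timeline.
; Separate per-hat Proyectil macros exist but are not called here.
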(event Custom|RotacionCamera
  (bind _newtrack_1 (Timeline|Timeline_0 Play)
    (:Update
      (Transformation|SetWorldRotation (Variables|Default|GetMierda) (Math|Rotator|MakeRotator 0.0 (.y _newtrack_1) 0.0) false false))))

(event EventBeginPlay
  (Utilities|FlowControl|Sequence
    (:then_0
      (Utilities|FlowControl|Delay 2.5)
      (Rendering|SetVisibility (Variables|Default|GetBola) false false)
      (Actor|DestroyActor))
    (:then_1
      (bind _aspc_paloma (Utilities|Casting|CastToPC_Paloma (Game|GetPlayerController 0)))
      (Variables|Default|SetRef%20PCPAloma _aspc_paloma))
    (:then_2
      (Utilities|FlowControl|Sequence
        (:then_1
          (Utilities|Proyectiles))))))

(fn ConstructionScript)

(fn RestablecerAnimacionShitNormal
  (bind _mierda (Variables|Default|GetMierda))
  (if (== (Variables|/Script/Engine.SkinnedMeshComponent|GetSkeletalMesh _mierda) "/Game/BluePrints/Proyectil/AnimationShit.AnimationShit")
    (Class|SkinnedMeshComponent|SetSkeletalMesh _mierda "/Game/BluePrints/Proyectil/AnimationShit.AnimationShit" true)
    (Components|SkeletalMesh|SetAnimInstanceClass _mierda "/Game/BluePrints/Proyectil/ShitAnimBP.ShitAnimBP_C")))