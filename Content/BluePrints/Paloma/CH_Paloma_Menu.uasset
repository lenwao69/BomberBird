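; CH_Paloma_Menu is the menu version of the Paloma pigeon, displaying a chosen hat and skin texture.
; Update_Paloma_Menu looks up a row name in DataTable_Gorros, then shows the Gorro component with that row's static mesh.
; It also applies the row's texture to the body through a new dynamic instance of Mat_Pidgeon_Basic on each successful lookup.
; BeginPlay caches the PC_Paloma player controller, which is not otherwise used here.
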(event Custom|Update_Paloma_Menu
  (params (RowName :type Name))
  (bind _gorro (Variables|Default|GetGorro))
  (bind _returnvalue (Utilities|GetDataTableRow "/Game/Structure/DataTable_Gorros.DataTable_Gorros" RowName)
    (:then
      (Rendering|SetVisibility _gorro true false)
      (Components|StaticMesh|SetStaticMesh _gorro (.Gorro (Utilities|Struct|BreakStruct_Gorros _returnvalue)))
      (bind _returnvalue_2 (Rendering|Material|CreateDynamicMaterialInstance (Variables|Character|GetMesh) 0 "/Game/Materials/Mat_Pidgeon_Basic.Mat_Pidgeon_Basic" "None" :!class /Script/Engine.PrimitiveComponent))
      (Rendering|Material|SetTextureParameterValue _returnvalue_2 "Texture_Pidg" (.Textura (Utilities|Struct|BreakStruct_Gorros _returnvalue))))))

(event EventBeginPlay
  (bind _aspc_paloma (Utilities|Casting|CastToPC_Paloma (Game|GetPlayerController 0)))
  (Variables|Default|SetRef_PC_Paloma _aspc_paloma))

(fn ConstructionScript)