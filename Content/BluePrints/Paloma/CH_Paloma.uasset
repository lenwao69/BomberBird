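; CH_Paloma is the pigeon character, handling game start-up screens, cosmetic appearance and a flee move.
; BeginPlay caches the PC_Paloma controller, shows a loading widget for a second, then pauses and opens the start menu.
; Update_Paloma_CH uses the controller's equipped hat to set hat mesh and body texture from DataTable_Gorros via a dynamic material, hiding the hat for "Basic".
; Huir moves the capsule to R's location over one second.
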(event Custom|Huir
  (Components|MoveComponentTo (Variables|Collision|GetCapsuleComponent) (Transformation|GetWorldLocation (Variables|Default|GetR)) (Transformation|GetWorldRotation (Variables|Character|GetMesh)) false false 1.0 false))

(event Custom|Update_Paloma_CH
  (bind _ref_pc_paloma (Variables|Default|GetRef_PC_Paloma))
  (bind _gorro (Variables|Default|GetGorro))
  (bind _gorro_equipado (Variables|/Game/BluePrints/Paloma/PC_Paloma.PC_Paloma_C|GetGorro_Equipado _ref_pc_paloma))
  (bind _returnvalue (Utilities|GetDataTableRow "/Game/Structure/DataTable_Gorros.DataTable_Gorros" _gorro_equipado)
    (:then
      (Components|StaticMesh|SetStaticMesh _gorro (.Gorro (Utilities|Struct|BreakStruct_Gorros _returnvalue)))
      (if (Utilities|Name|Equal(Name) _gorro_equipado "Basic")
        (Rendering|SetVisibility _gorro false false)
        (else
          (Rendering|SetVisibility _gorro true false)))
      (bind _returnvalue_2 (Rendering|Material|CreateDynamicMaterialInstance (Variables|Character|GetMesh) 0 "/Game/Materials/Mat_Pidgeon_Basic.Mat_Pidgeon_Basic" "None" :!class /Script/Engine.PrimitiveComponent))
      (Rendering|Material|SetTextureParameterValue _returnvalue_2 "Texture_Pidg" (.Textura (Utilities|Struct|BreakStruct_Gorros _returnvalue))))))

(event EventBeginPlay
  (bind _aspc_paloma (Utilities|Casting|CastToPC_Paloma (Game|GetPlayerController 0)))
  (Variables|Default|SetRef_PC_Paloma _aspc_paloma)
  (bind _returnvalue (UserInterface|CreateWidget "/Game/Widgets/Menu/Widg_Loading.Widg_Loading_C"))
  (UserInterface|Viewport|AddtoViewport _returnvalue 0)
  (Utilities|FlowControl|Delay 1.0)
  (Game|SetGamePaused true)
  (Widget|RemovefromParent _returnvalue)
  (bind _returnvalue_2 (UserInterface|CreateWidget "/Game/Widgets/HUD/Widg_Start.Widg_Start_C"))
  (UserInterface|Viewport|AddtoViewport _returnvalue_2 0))

(fn ConstructionScript)